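; BP_Knife is a knife actor that can be picked up and dropped through events.
; BeginPlay and EPickup share one path that, when IsAttached is false, enables physics simulation on the knife mesh and attaches the root component to the pickup's Parent, keeping relative transforms.
; EDrop disables physics simulation and detaches the actor, keeping its world transform.
; IsAttached is only read here, never set.
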(event Custom|EPickup
  (params (Parent :type Scene%20Component%20Object%20Reference))
  (if (not (Variables|Default|GetIsAttached))
    (Physics|SetSimulatePhysics (Variables|Default|GetKnifeMesh) true)
    (Transformation|AttachComponentToComponent (VehicleSound|GetRootComponent) Parent "None" "KeepRelative" "KeepRelative" "KeepRelative" true)))

(event Custom|EDrop
  (Physics|SetSimulatePhysics (Variables|Default|GetKnifeMesh) false)
  (Transformation|DetachFromActor "KeepWorld" "KeepWorld" "KeepWorld"))

(event EventBeginPlay
  (if (not (Variables|Default|GetIsAttached))
    (Physics|SetSimulatePhysics (Variables|Default|GetKnifeMesh) true)
    (Transformation|AttachComponentToComponent (VehicleSound|GetRootComponent) (stale Custom|EPickup Parent) "None" "KeepRelative" "KeepRelative" "KeepRelative" true)))

(fn ConstructionScript)