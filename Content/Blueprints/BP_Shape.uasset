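; BP_Shape is a shape actor that can be picked up and dropped.
; Pickup, gated on not being attached, turns off the mesh's physics and collision, then attaches the root component to the supplied component, keeping its world transform.
; Drop restores physics simulation and collision, then detaches the actor in place.
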(event EventPickup
  (params (AttachTo :type Scene%20Component%20Object%20Reference))
  (bind _shapemesh (Variables|Default|GetShapeMesh))
  (if (not (Variables|Default|GetIsAttached))
    (Physics|SetSimulatePhysics _shapemesh false)
    (Collision|SetCollisionEnabled _shapemesh "NoCollision")
    (Transformation|AttachComponentToComponent (VehicleSound|GetRootComponent) AttachTo "None" "KeepWorld" "KeepWorld" "KeepWorld" false)))

(event EventDrop
  (bind _shapemesh (Variables|Default|GetShapeMesh))
  (Physics|SetSimulatePhysics _shapemesh true)
  (Collision|SetCollisionEnabled _shapemesh "QueryAndPhysics")
  (Transformation|DetachFromActor "KeepWorld" "KeepWorld" "KeepWorld"))

(fn ConstructionScript)