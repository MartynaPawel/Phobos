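; BP_Podium is a podium that accepts three numbered BP_Shape actors, each in its matching collision slot.
; An overlap with the right ShapeNumber marks the shape as attached, hides its mesh and reveals the podium's own mesh for that slot, faking the placement.
; Only shape 1 is then destroyed; the destroy calls for shapes 2 and 3 are disconnected, leaving those actors hidden in the level.
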(event OnComponentBeginOverlap(Collision1)
  (params (OverlappedComponent :type Primitive%20Component%20Object%20Reference) (OtherActor :type Actor%20Object%20Reference) (OtherComp :type Primitive%20Component%20Object%20Reference) (OtherBodyIndex :type Integer) (bFromSweep :type Boolean) (SweepResult :type Hit%20Result%20Structure%20%28by%20ref%29))
  (bind _asbp_shape (Utilities|Casting|CastToBP_Shape OtherActor))
  (if (== (Variables|/Game/Blueprints/BP_Shape.BP_Shape_C|GetShapeNumber _asbp_shape) 1)
    (Variables|/Game/Blueprints/BP_Shape.BP_Shape_C|SetIsAttached _asbp_shape true)
    (Rendering|SetVisibility (Variables|Default|GetShape1) true false)
    (Rendering|SetVisibility (Variables|/Game/Blueprints/BP_Shape.BP_Shape_C|GetShapeMesh _asbp_shape) false false)
    (Actor|DestroyActor _asbp_shape)))

(event OnComponentBeginOverlap(Collision2)
  (params (OverlappedComponent :type Primitive%20Component%20Object%20Reference) (OtherActor :type Actor%20Object%20Reference) (OtherComp :type Primitive%20Component%20Object%20Reference) (OtherBodyIndex :type Integer) (bFromSweep :type Boolean) (SweepResult :type Hit%20Result%20Structure%20%28by%20ref%29))
  (bind _asbp_shape (Utilities|Casting|CastToBP_Shape OtherActor))
  (if (== (Variables|/Game/Blueprints/BP_Shape.BP_Shape_C|GetShapeNumber _asbp_shape) 2)
    (Variables|/Game/Blueprints/BP_Shape.BP_Shape_C|SetIsAttached _asbp_shape true)
    (Rendering|SetVisibility (Variables|Default|GetShape2) true false)
    (Rendering|SetVisibility (Variables|/Game/Blueprints/BP_Shape.BP_Shape_C|GetShapeMesh _asbp_shape) false false)))

(event OnComponentBeginOverlap(Collision3)
  (params (OverlappedComponent :type Primitive%20Component%20Object%20Reference) (OtherActor :type Actor%20Object%20Reference) (OtherComp :type Primitive%20Component%20Object%20Reference) (OtherBodyIndex :type Integer) (bFromSweep :type Boolean) (SweepResult :type Hit%20Result%20Structure%20%28by%20ref%29))
  (bind _asbp_shape (Utilities|Casting|CastToBP_Shape OtherActor))
  (if (== (Variables|/Game/Blueprints/BP_Shape.BP_Shape_C|GetShapeNumber _asbp_shape) 3)
    (Variables|/Game/Blueprints/BP_Shape.BP_Shape_C|SetIsAttached _asbp_shape true)
    (Rendering|SetVisibility (Variables|Default|GetShape3) true false)
    (Rendering|SetVisibility (Variables|/Game/Blueprints/BP_Shape.BP_Shape_C|GetShapeMesh _asbp_shape) false false)))

(fn ConstructionScript)