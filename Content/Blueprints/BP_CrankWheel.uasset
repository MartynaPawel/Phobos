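; BP_CrankWheel is a crank wheel actor that can be picked up and dropped.
; Pickup checks that IsAttached is false, then turns off physics and collision on CrankWMesh and attaches the root to the supplied component, keeping world transform.
; Drop restores physics and collision and detaches the actor in place.
; Neither event updates IsAttached, and the construction script is empty.
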(event EventPickup
  (params (AttachTo :type Scene%20Component%20Object%20Reference))
  (bind _crankwmesh (Variables|Default|GetCrankWMesh))
  (if (not (Variables|Default|GetIsAttached))
    (Physics|SetSimulatePhysics _crankwmesh false)
    (Collision|SetCollisionEnabled _crankwmesh "NoCollision")
    (Transformation|AttachComponentToComponent (VehicleSound|GetRootComponent) AttachTo "None" "KeepWorld" "KeepWorld" "KeepWorld" false)))

(event EventDrop
  (bind _crankwmesh (Variables|Default|GetCrankWMesh))
  (Physics|SetSimulatePhysics _crankwmesh true)
  (Collision|SetCollisionEnabled _crankwmesh "QueryAndPhysics")
  (Transformation|DetachFromActor "KeepWorld" "KeepWorld" "KeepWorld"))

(fn ConstructionScript)