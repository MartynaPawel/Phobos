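; BP_RisingWater2 is a water actor that moves along a referenced spline track.
; If active, it calls MoveActor on BeginPlay, which proceeds only if the FirstPersonCharacter's first objective is already complete.
; A timeline, scaled by Duration and offset by ActorStartOffset, lerps distance along the spline to set world location and rotation.
; A disconnected BP_VRChar cast marks an intended replacement for the character check.
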(event Custom|MoveActor
  (bind _asfirst_person_character (Utilities|Casting|CastToFirstPersonCharacter (Game|GetPlayerCharacter 0)))
  (if (Variables|/Game/FirstPersonBP/Blueprints/FirstPersonCharacter.FirstPersonCharacter_C|GetOBJ1Complete _asfirst_person_character)
    (Components|Timeline|SetPlayRate (Variables|Default|GetTimeline_0) (/ 1.0 (Variables|Default|GetDuration)))
    (Components|Timeline|SetNewTime (Variables|Default|GetTimeline_0) (Variables|Default|GetActorStartOffset))
    (bind _alpha (Timeline|Timeline_0 Play)
      (:Update
        (Variables|Default|SetAlpha _alpha)
        (Transformation|SetActorLocationAndRotation (Spline|GetLocationatDistanceAlongSpline (Variables|/Game/Blueprints/BP_Track.BP_Track_C|GetSpline (Variables|Default|GetTrackRef)) (Math|Float|Lerp 0.0 (Spline|GetSplineLength (Variables|/Game/Blueprints/BP_Track.BP_Track_C|GetSpline (Variables|Default|GetTrackRef))) (Variables|Default|GetAlpha)) "World") (Spline|GetRotationatDistanceAlongSpline (Variables|/Game/Blueprints/BP_Track.BP_Track_C|GetSpline (Variables|Default|GetTrackRef)) (Math|Float|Lerp 0.0 (Spline|GetSplineLength (Variables|/Game/Blueprints/BP_Track.BP_Track_C|GetSpline (Variables|Default|GetTrackRef))) (Variables|Default|GetAlpha)) "World"))))))

(event EventBeginPlay
  (if (Variables|Default|GetActiveActor)
    (CallFunction|MoveActor)))

(fn ConstructionScript)