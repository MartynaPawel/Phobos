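; BP_Key is a physical key actor that can be picked up and dropped.
; Pickup checks that IsAttached is false, then turns off the mesh's physics and collision and attaches the root to the given component, keeping its world transform.
; Drop restores physics and query-and-physics collision, then detaches the actor in place.
; The file only reads IsAttached and never sets it.
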(event EventPickup
  (params (AttachTo :type Scene%20Component%20Object%20Reference))
  (bind _keymesh (Variables|Default|GetKeyMesh))
  (if (not (Variables|Default|GetIsAttached))
    (Physics|SetSimulatePhysics _keymesh false)
    (Collision|SetCollisionEnabled _keymesh "NoCollision")
    (Transformation|AttachComponentToComponent (VehicleSound|GetRootComponent) AttachTo "None" "KeepWorld" "KeepWorld" "KeepWorld" false)))

(event EventDrop
  (bind _keymesh (Variables|Default|GetKeyMesh))
  (Physics|SetSimulatePhysics _keymesh true)
  (Collision|SetCollisionEnabled _keymesh "QueryAndPhysics")
  (Transformation|DetachFromActor "KeepWorld" "KeepWorld" "KeepWorld"))

(fn ConstructionScript)