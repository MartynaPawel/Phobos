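; BP_WebDoor is a cobweb obstacle, named as a door, that the knife clears to complete the fifth objective.
; When a BP_Knife overlaps its Collision component, it plays a cobweb break sound and hides the three web components.
; It then sets OBJ5Complete on the FirstPersonCharacter; an equivalent branch for BP_VRChar is present but never runs.
; The Collision component is left untouched, so later knife overlaps repeat the sequence.
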(event OnComponentBeginOverlap(Collision)
  (params (OverlappedComponent :type Primitive%20Component%20Object%20Reference) (OtherActor :type Actor%20Object%20Reference) (OtherComp :type Primitive%20Component%20Object%20Reference) (OtherBodyIndex :type Integer) (bFromSweep :type Boolean) (SweepResult :type Hit%20Result%20Structure%20%28by%20ref%29))
  (Utilities|Casting|CastToBP_Knife OtherActor)
  (Audio|PlaySound2D "/Game/SFX/CobwebBreak_Cue.CobwebBreak_Cue" 1.0 1.0 0.0 0 0)
  (Rendering|SetVisibility (Variables|Default|GetCobWeb) false false)
  (bind _asfirst_person_character (Utilities|Casting|CastToFirstPersonCharacter (Game|GetPlayerCharacter 0)))
  (Variables|/Game/FirstPersonBP/Blueprints/FirstPersonCharacter.FirstPersonCharacter_C|SetOBJ5Complete _asfirst_person_character true))

(fn ConstructionScript)