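; BP_LockedDoor is a VR door lock that accepts a BP_Key and completes the player's third objective.
; When a key overlaps the CollisionHole, it is destroyed and a stand-in key mesh on the door becomes visible.
; After a short delay the lock plays a turn sound, snaps that mesh to a rotated angle and sets the objective flag on BP_VRChar.
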(event OnComponentBeginOverlap(CollisionHole)
  (params (OverlappedComponent :type Primitive%20Component%20Object%20Reference) (OtherActor :type Actor%20Object%20Reference) (OtherComp :type Primitive%20Component%20Object%20Reference) (OtherBodyIndex :type Integer) (bFromSweep :type Boolean) (SweepResult :type Hit%20Result%20Structure%20%28by%20ref%29))
  (bind _asbp_key (Utilities|Casting|CastToBP_Key OtherActor))
  (Development|PrintString "Hello")
  (Variables|/Game/Blueprints/BP_Key.BP_Key_C|SetIsAttached _asbp_key true)
  (Rendering|SetVisibility (Variables|Default|GetKeyMesh2) true false)
  (Rendering|SetVisibility (Variables|/Game/Blueprints/BP_Key.BP_Key_C|GetKeyMesh _asbp_key) false false)
  (Actor|DestroyActor _asbp_key)
  (Utilities|FlowControl|Delay 1.0)
  (Audio|PlaySound2D "/Game/SFX/KeyTurn_Cue.KeyTurn_Cue" 1.0 1.0 0.0 0 0)
  (Transformation|SetWorldRotation (Variables|Default|GetKeyMesh2) "0.000000,45.000000,0.000000" false false)
  (bind _asbp_vrchar (Utilities|Casting|CastToBP_VRChar (Game|GetPlayerCharacter 0)))
  (Variables|/Game/PlayerChar/BP_VRChar.BP_VRChar_C|SetObjective3Complete _asbp_vrchar true))

(fn ConstructionScript)